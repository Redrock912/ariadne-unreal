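; DirectionActor is a paper sprite actor that blinks in game, likely serving as a direction indicator.
; Tick accumulates DeltaSeconds into FlickerTime until it exceeds FlickLimit.
; A FlipFlop then alternately hides and shows the PaperSprite component and resets the timer, producing a steady flicker.
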(event `self.ReceiveTick`
  (params (DeltaSeconds :type "Float (single-precision)"))
  (bind _papersprite (`self.PaperSprite`))
  (bind _output_get (set `self.flickerTime` (+ (`self.flickerTime`) DeltaSeconds)))
  (if (> _output_get (`self.flickLimit`))
    (`/Engine/EditorBlueprintResources/StandardMacros.FlipFlop`
      (:`A`
        (`SceneComponent.SetHiddenInGame` _papersprite true false)
        (set `self.flickerTime` 0.0))
      (:`B`
        (`SceneComponent.SetHiddenInGame` _papersprite false false)
        (set `self.flickerTime` 0.0)))))

(fn `UserConstructionScript`)