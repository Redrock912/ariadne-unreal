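; DoorActor is a door Actor that swings open and closed when its ToggleDoor event is called.
; ToggleDoor plays a timeline forward from the start or reverses it from the end, depending on the Opened flag.
; The timeline track, scaled by OpenAngle, drives the Door component's relative yaw.
; Opened flips only when the timeline finishes, alongside a debug "Hello" print.
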(event `ToggleDoor`
  (if (`self.Opened`)
    (bind (_direction `_새_트랙_0`) (`Timeline|타임라인_0` :!via `ReverseFromEnd` :!label _label)
      (:`Update`
        (`SceneComponent.K2_SetRelativeRotation` (`self.Door`) (`KismetMathLibrary.MakeRotator` 0.0 0.0 (* `_새_트랙_0` (`self.OpenAngle`))) false false))
      (:`Finished`
        (`KismetSystemLibrary.PrintString` "Hello")
        (set `self.Opened` (not (`self.Opened`)))))
    (else
      (goto _label :!via `PlayFromStart`))))

(fn `UserConstructionScript`)