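; Dot actor with a sphere that absorbs other dots it touches and takes one of four random pastel colors.
; The construction script creates a dynamic material instance and sets its Color through chained random rolls, so the four colors are not equally likely.
; On sphere overlap with another dotActor, it destroys that dot and sets IsMerge.
; A node to spawn a dot at the sphere's location is left unconnected.
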(event `self.Sphere.OnComponentBeginOverlap`
  (params (OverlappedComponent :type "PrimitiveComponent Object Reference") (OtherActor :type "Actor Object Reference") (OtherComp :type "PrimitiveComponent Object Reference") (OtherBodyIndex :type Integer) (bFromSweep :type Boolean) (SweepResult :type "HitResult Structure (by ref)"))
  (bind _asdot_actor (cast `/Game/Blueprints/Actors/dotActor` OtherActor))
  (`self.K2_DestroyActor` _asdot_actor)
  (set `self.isMerge` true))

(fn `UserConstructionScript`
  (bind _returnvalue (`KismetMathLibrary.RandomFloatInRange` 0.0 1.0))
  (bind _dmi (`self.DMI`))
  (bind _returnvalue_2 (`PrimitiveComponent.CreateDynamicMaterialInstance` (`self.Sphere`) 0 null))
  (set `self.DMI` _returnvalue_2)
  (if (> _returnvalue 0.75)
    (`MaterialInstanceDynamic.SetVectorParameterValue` _dmi "Color" (`KismetMathLibrary.MakeColor` 0.3 1.0 0.5))
    (elif (> _returnvalue 0.5)
      (`MaterialInstanceDynamic.SetVectorParameterValue` _dmi "Color" (`KismetMathLibrary.MakeColor` 0.4 1.0 1.0))
      (elif (> _returnvalue 0.25)
        (`MaterialInstanceDynamic.SetVectorParameterValue` _dmi "Color" (`KismetMathLibrary.MakeColor` 1.0 0.6 1.0))
        (else
          (`MaterialInstanceDynamic.SetVectorParameterValue` _dmi "Color" (`KismetMathLibrary.MakeColor` 1.0 1.0 0.6)))))))