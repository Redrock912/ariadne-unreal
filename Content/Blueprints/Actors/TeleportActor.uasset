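; TeleportActor is a door actor that loads the WoodMap level when its swing animation finishes.
; OpenDoor plays or reverses a timeline that scales OpenAngle into the Door's yaw, then toggles Opened and opens the level.
; CloseDoor stops and resets the timeline, and Cube hits print a debug string.
; A disconnected chain would spawn a delayed snow particle after checking the player's view angle toward the actor.
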(event `self.ReceiveBeginPlay`)

(event `self.ReceiveTick`
  (params (DeltaSeconds :type "Float (single-precision)")))

(event `OpenDoor`
  (if (not (`TimelineComponent.IsPlaying` (`self.타임라인_0`)))
    (if (`self.Opened`)
      (bind (_direction `_새_트랙_0`) (`Timeline|타임라인_0` :!via `ReverseFromEnd` :!label _label)
        (:`Update`
          (`SceneComponent.K2_SetRelativeRotation` (`self.Door`) (`KismetMathLibrary.MakeRotator` 0.0 0.0 (* `_새_트랙_0` (`self.OpenAngle`))) false false))
        (:`Finished`
          (`KismetSystemLibrary.PrintString` "Hello")
          (set `self.Opened` (not (`self.Opened`)))
          (`GameplayStatics.OpenLevel` "WoodMap")))
      (else
        (goto _label :!via `PlayFromStart`)))))

(event `CloseDoor`
  (`|ExecutionSequence`
    (:`then_0`
      (goto _label :!via `Stop`))
    (:`then_1`
      (goto _label :!via `SetNewTime`))))

(event `self.Cube.OnComponentHit`
  (params (HitComponent :type "PrimitiveComponent Object Reference") (OtherActor :type "Actor Object Reference") (OtherComp :type "PrimitiveComponent Object Reference") (NormalImpulse :type "Vector Structure") (Hit :type "HitResult Structure (by ref)"))
  (`KismetSystemLibrary.PrintString` "Hello"))

(fn `UserConstructionScript`)