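; Floor UI actor that turns in yaw to follow player 0's camera control rotation once it drifts more than 30 degrees away.
; Tick converts actor yaw to 0–360 via TransformActorRot and wraps the difference to the shortest turn.
; The BackToControlView timeline then scales that delta to rotate the actor, pausing drift checks until finished.
; Debug prints, disconnected rotation experiments and an uncalled SetActorRot function remain.
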(event EventTick
  (params (DeltaSeconds :type Float%20%28single-precision%29))
  (Utilities|FlowControl|Sequence
    (:then_0
      (Utilities|FlowControl|DoOnce false
        (:Completed
          (Variables|Default|SetLastControlYaw (Variables|Default|GetCurrentControlYaw)))))
    (:then_1
      (if (Variables|Default|GetMoving)
        (bind _float (Timeline|BackToControlView Play)
          (:Update
            (Development|PrintString (Utilities|String|ToString(Float) (* _float (Variables|Default|GetDelta))))
            (Transformation|SetActorRotation (Math|Rotator|MakeRotator 0.0 0.0 (+ (Variables|Default|GetActorYaw) (* _float (Variables|Default|GetDelta))))))
          (:Finished
            (Variables|Default|SetMoving false)
            (Development|PrintString "Hello")))
        (else
          ;[1 1 1] 입력(input) 데이터
          (Variables|Default|SetCurrentControlYaw (.Yaw (Math|Rotator|BreakRotator (Pawn|GetControlRotation (Game|GetPlayerController 0) :!class /Script/Engine.Controller))))
          (Variables|Default|SetActorYaw (CallFunction|TransformActorRot (.yaw (Transformation|GetActorRotation))))
          ;[1 1 1] Delta 값 설정
          (bind _output_get (Variables|Default|SetDelta (- (Variables|Default|GetCurrentControlYaw) (Variables|Default|GetActorYaw))))
          (if (> (Math|Float|Absolute(Float) _output_get) 1.8e+02)
            (Variables|Default|SetDelta (+ _output_get (* (/ _output_get (Math|Float|Absolute(Float) _output_get)) -3.6e+02))))
          (if (> (Math|Float|Absolute(Float) (Variables|Default|GetDelta)) 3e+01)
            (Variables|Default|SetMoving true)
            (Components|Timeline|SetNewTime (Variables|Default|GetBackToControlView) 0.0)))))))

(event EventBeginPlay)

(fn ConstructionScript)

(fn SetActorRot
  (params (0to360 :type Float%20%28single-precision%29))
  (if (>= 0to360 1.8e+02)
    (LocalVariables|SetTransformed -179.0)
    (else
      (LocalVariables|SetTransformed 0to360)))
  (Transformation|SetActorRotation (Math|Rotator|MakeRotator 0.0 0.0 (LocalVariables|GetTransformed))))

(fn TransformActorRot
  (params (Original :type Float%20%28single-precision%29))
  (return (select (Math|Float|InRange(Float) Original -1.8e+02 0.0 true false) (Math|Float|MapRangeClamped Original -1.8e+02 0.0 1.8e+02 3.6e+02) Original)))